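; Resource manager actor that tracks the player's stock of eight resource types and handles the costs of placing buildings and props.
; CanBuildActor maps the actor class to a cost array, compares it element-wise with the stock and prints any shortfall.
; UsingResourcesToBuildActor subtracts that cost, then updates the HUD.
; Tick copies values back from the HUD, reached through PlayerCameraPawn, so HUD-side changes overwrite the stock.
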(event `self.ReceiveTick`
  (params (DeltaSeconds :type "Float (single-precision)"))
  (`self.GetHUDResources`))

(event `self.ReceiveBeginPlay`
  (`self.SetHUD_Ref`)
  (`self.UpdateHUDResources`))

(fn `CanBuildActor`
  (params (ActorClass :type "Actor Class Reference"))
  (returns (HaveEnoughResources :type Boolean))
  (locals (Actor :type "Actor Class Reference") (isOK :type Boolean :default true) (BuildingResourcesArray :type "Array of Integer"))
  (set `local.Actor` ActorClass)
  ;[1 1 1] SwitchByActorClass
  ;;[1 1 1] cottage
  (if (== (`local.Actor`) "/Game/Blueprints/Spawning/Buildings/BP_TestCottageActor.BP_TestCottageActor_C")
    (set `local.BuildingResourcesArray` (`self.CottageResources`))
    (bind _isallgreaterorequal (`self.CompareArrays` (`self.Resources`) (`local.BuildingResourcesArray`) :!label _label))
    (if _isallgreaterorequal
      (set `self.isBuildingEnabled` true)
      (else
        (`self.PrintResourceMessage` (`local.Actor`) (`local.BuildingResourcesArray`) (`self.Resources`))
        (set `self.isBuildingEnabled` false :!label _label_2)))
    (else
      ;;[1 1 1] Cube
      (if (== (`local.Actor`) "/Game/Blueprints/Spawning/Objects/BP_TestCubeActor.BP_TestCubeActor_C")
        (set `local.BuildingResourcesArray` (`self.CubeResources`))
        (goto _label)
        (else
          ;;[1 1 1] castle
          (if (== (`local.Actor`) "/Game/Blueprints/Spawning/Buildings/Castle.Castle_C")
            (set `local.BuildingResourcesArray` (`self.CastleResources`))
            (goto _label)
            (else
              ;;[1 1 1] Factory
              (if (== (`local.Actor`) "/Game/Blueprints/Spawning/Buildings/Factory.Factory_C")
                (set `local.BuildingResourcesArray` (`self.FactoryResources`))
                (goto _label)
                (else
                  ;;[1 1 1] barrel
                  (if (== (`local.Actor`) "/Game/Blueprints/Spawning/Objects/Barrel.Barrel_C")
                    (set `local.BuildingResourcesArray` (`self.BarrelResources`))
                    (goto _label)
                    (else
                      ;;[1 1 1] catapult
                      (if (== (`local.Actor`) "/Game/Blueprints/Spawning/Objects/Catapult.Catapult_C")
                        (set `local.BuildingResourcesArray` (`self.CatapultResources`))
                        (goto _label)
                        (else
                          ;;[1 1 1] cauldron
                          (if (== (`local.Actor`) "/Game/Blueprints/Spawning/Objects/Cauldron.Cauldron_C")
                            (set `local.BuildingResourcesArray` (`self.CauldronResources`))
                            (goto _label)
                            (else
                              ;;[1 1 1] chest
                              (if (== (`local.Actor`) "/Game/Blueprints/Spawning/Objects/Chest.Chest_C")
                                (set `local.BuildingResourcesArray` (`self.ChestResources`))
                                (goto _label)
                                (else
                                  ;;[1 1 1] nothing
                                  (if (== (`local.Actor`) null)
                                    (goto _label_2)
                                    (else
                                      (`KismetSystemLibrary.PrintString` "INTERNAL ERROR: Unknown Actor Type!" true true (struct :`R` 1.0 :`A` 1.0))
                                      (goto _label_2)))))))))))))))))))
  (return (`self.isBuildingEnabled`)))

(fn `CompareArrays`
  (params (ResourceArray :type "Array of Integer") (BuildingResourceArray :type "Array of Integer"))
  (returns (isAllGreaterOrEqual :type Boolean))
  (locals (ok :type Boolean :default true))
  (for (_array_element _array_index) ResourceArray
    (set `local.ok` (and (>= _array_element (`KismetArrayLibrary.Array_Get` BuildingResourceArray _array_index)) (`local.ok`))))
  (return (`local.ok`)))

(fn `GetHUDResources`
  (bind _hud_ref (`self.Hud_Ref`))
  (`KismetArrayLibrary.Array_Set` (`self.Resources`) (`self.MeatIndex`) (`/Game/Blueprints/GUI/HUD.meatValue` _hud_ref))
  (`KismetArrayLibrary.Array_Set` (`self.Resources`) (`self.WaterIndex`) (`/Game/Blueprints/GUI/HUD.waterValue` _hud_ref))
  (`KismetArrayLibrary.Array_Set` (`self.Resources`) (`self.WheatIndex`) (`/Game/Blueprints/GUI/HUD.wheatValue` _hud_ref))
  (`KismetArrayLibrary.Array_Set` (`self.Resources`) (`self.FruitIndex`) (`/Game/Blueprints/GUI/HUD.fruitValue` _hud_ref))
  (`KismetArrayLibrary.Array_Set` (`self.Resources`) (`self.WoodIndex`) (`/Game/Blueprints/GUI/HUD.woodValue` _hud_ref))
  (`KismetArrayLibrary.Array_Set` (`self.Resources`) (`self.StoneIndex`) (`/Game/Blueprints/GUI/HUD.stoneValue` _hud_ref))
  (`KismetArrayLibrary.Array_Set` (`self.Resources`) (`self.IronIndex`) (`/Game/Blueprints/GUI/HUD.ironValue` _hud_ref))
  (`KismetArrayLibrary.Array_Set` (`self.Resources`) (`self.SandIndex`) (`/Game/Blueprints/GUI/HUD.sandValue` _hud_ref)))

(fn `PrintResourceMessage`
  (params (ActorClass :type "Actor Class Reference") (NeededResourcesArray :type "Array of Integer") (ResourcesArray :type "Array of Integer"))
  (locals (WoodString :type String) (StoneString :type String) (IronString :type String) (SandString :type String) (BuildingTypeString :type String) (DifferenceArray :type "Array of Integer") (ResStringArray :type "Array of String") (MeatString :type String) (WaterString :type String) (WheatString :type String) (FruitString :type String))
  (bind _resstringarray (`local.ResStringArray`))
  (bind _output_get (set `local.DifferenceArray` NeededResourcesArray))
  (`self.SubtractArrayElements` _output_get ResourcesArray
    (:`Completed`
      (for (_array_element _array_index) (`local.DifferenceArray`)
        (if (> _array_element 0)
          (`KismetArrayLibrary.Array_Set` _resstringarray _array_index (`KismetStringLibrary.Conv_IntToString` _array_element))))
      (for (_array_element_2 _array_index_2) _resstringarray
        (if (`KismetStringLibrary.NotEqual_StrStr` _array_element_2)
          (switch `int` _array_index_2
            (:`0`
              (set `local.MeatString` (`KismetStringLibrary.Concat_StrStr` _array_element_2 " more meat ")))
            (:`1`
              (set `local.WaterString` (`KismetStringLibrary.Concat_StrStr` _array_element_2 " more water ")))
            (:`2`
              (set `local.WheatString` (`KismetStringLibrary.Concat_StrStr` _array_element_2 " more wheat ")))
            (:`3`
              (set `local.FruitString` (`KismetStringLibrary.Concat_StrStr` _array_element_2 " more fruit ")))
            (:`4`
              (set `local.WoodString` (`KismetStringLibrary.Concat_StrStr` _array_element_2 " more wood ")))
            (:`5`
              (set `local.StoneString` (`KismetStringLibrary.Concat_StrStr` _array_element_2 " more stone ")))
            (:`6`
              (set `local.IronString` (`KismetStringLibrary.Concat_StrStr` _array_element_2 " more iron ")))
            (:`7`
              (set `local.SandString` (`KismetStringLibrary.Concat_StrStr` _array_element_2 " more sand "))))))
      (bind _buildingtype (`self.DefineBuildingType` ActorClass))
      (set `local.BuildingTypeString` _buildingtype)
      (`KismetSystemLibrary.PrintString` (`KismetStringLibrary.Concat_StrStr` "You need " (`local.MeatString`) (`local.WaterString`) (`local.WheatString`) (`local.FruitString`) (`local.WoodString`) (`local.StoneString`) (`local.IronString`) (`local.SandString`) " to make a " (`local.BuildingTypeString`) "!") true true (struct :`R` 1.0 :`A` 1.0) 10.0))))

(fn `UpdateHUDResources`
  (`self.SetHUD_Ref`)
  (`|ExecutionSequence`
    (:`then_0`
      (set `/Game/Blueprints/GUI/HUD.meatValue` (`KismetArrayLibrary.Array_Get` (`self.Resources`) (`self.MeatIndex`)) (`self.Hud_Ref`)))
    (:`then_1`
      (set `/Game/Blueprints/GUI/HUD.waterValue` (`KismetArrayLibrary.Array_Get` (`self.Resources`) (`self.WaterIndex`)) (`self.Hud_Ref`)))
    (:`then_2`
      (set `/Game/Blueprints/GUI/HUD.wheatValue` (`KismetArrayLibrary.Array_Get` (`self.Resources`) (`self.WheatIndex`)) (`self.Hud_Ref`)))
    (:`then_3`
      (set `/Game/Blueprints/GUI/HUD.fruitValue` (`KismetArrayLibrary.Array_Get` (`self.Resources`) (`self.FruitIndex`)) (`self.Hud_Ref`)))
    (:`then_4`
      (set `/Game/Blueprints/GUI/HUD.woodValue` (`KismetArrayLibrary.Array_Get` (`self.Resources`) (`self.WoodIndex`)) (`self.Hud_Ref`)))
    (:`then_5`
      (set `/Game/Blueprints/GUI/HUD.stoneValue` (`KismetArrayLibrary.Array_Get` (`self.Resources`) (`self.StoneIndex`)) (`self.Hud_Ref`)))
    (:`then_6`
      (set `/Game/Blueprints/GUI/HUD.ironValue` (`KismetArrayLibrary.Array_Get` (`self.Resources`) (`self.IronIndex`)) (`self.Hud_Ref`)))
    (:`then_7`
      (set `/Game/Blueprints/GUI/HUD.sandValue` (`KismetArrayLibrary.Array_Get` (`self.Resources`) (`self.SandIndex`)) (`self.Hud_Ref`)))))

(fn `UserConstructionScript`)

(fn `UsingResourcesToBuildActor`
  (params (ActorClass :type "Actor Class Reference"))
  (locals (BuildingResourceArray :type "Array of Integer"))
  ;[1 1 1] cottage resources
  (if (== ActorClass "/Game/Blueprints/Spawning/Buildings/BP_TestCottageActor.BP_TestCottageActor_C")
    (set `local.BuildingResourceArray` (`self.CottageResources`))
    (`self.SubtractArrayElements` (`self.Resources`) (`local.BuildingResourceArray`) :!label _label
      (:`Completed`
        (`self.UpdateHUDResources`)))
    (else
      ;[1 1 1] cube resources
      (if (== ActorClass "/Game/Blueprints/Spawning/Objects/BP_TestCubeActor.BP_TestCubeActor_C")
        (set `local.BuildingResourceArray` (`self.CubeResources`))
        (goto _label)
        (else
          ;[1 1 1] Castle resources
          (if (== ActorClass "/Game/Blueprints/Spawning/Buildings/Castle.Castle_C")
            (set `local.BuildingResourceArray` (`self.CastleResources`))
            (goto _label)
            (else
              ;[1 1 1] factory resources
              (if (== ActorClass "/Game/Blueprints/Spawning/Buildings/Factory.Factory_C")
                (set `local.BuildingResourceArray` (`self.FactoryResources`))
                (goto _label)
                (else
                  ;[1 1 1] barrel resources
                  (if (== ActorClass "/Game/Blueprints/Spawning/Objects/Barrel.Barrel_C")
                    (set `local.BuildingResourceArray` (`self.BarrelResources`))
                    (goto _label)
                    (else
                      ;[1 1 1] ctapult resources
                      (if (== ActorClass "/Game/Blueprints/Spawning/Objects/Catapult.Catapult_C")
                        (set `local.BuildingResourceArray` (`self.CatapultResources`))
                        (goto _label)
                        (else
                          ;[1 1 1] Cauldron resources
                          (if (== ActorClass "/Game/Blueprints/Spawning/Objects/Cauldron.Cauldron_C")
                            (set `local.BuildingResourceArray` (`self.CauldronResources`))
                            (goto _label)
                            (else
                              ;[1 1 1] chest resources
                              (if (== ActorClass "/Game/Blueprints/Spawning/Objects/Chest.Chest_C")
                                (set `local.BuildingResourceArray` (`self.ChestResources`))
                                (goto _label)
                                (else
                                  ;[1 1 1] nothing
                                  (if (not (== ActorClass null))
                                    (`KismetSystemLibrary.PrintString` "INTERNAL ERROR: Unknown Actor Type!" true true (struct :`R` 1.0 :`A` 1.0)))))))))))))))))))
  (return))