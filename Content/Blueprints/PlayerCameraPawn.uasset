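; Player pawn for a top-down building game camera, with axis movement, wheel zoom, right-drag rotation and screen-edge scrolling.
; Movement funnels through CalculateAndSetActorTransform, which clamps position to the Floor actor's bounds.
; BeginPlay creates a hidden HUD and spawns a ResourceManager; Tick keeps the minimap camera following the pawn.
; Left click line-traces under the cursor to spawn ActorClass, subject to resource and collision checks, then charges resources.
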(event `self.ReceiveBeginPlay`
  (bind (_returnvalue_x _returnvalue_y) (`KismetMathLibrary.BreakVector` (`SceneComponent.K2_GetComponentLocation` (`self.Scene`))))
  ;[1 1 1] BeginPlay operations
  (`|ExecutionSequence`
    (:`then_0`
      ;;[1 1 1] Set world bounds
      (set `self.maxDistanceY` (.y (`.BoxExtent` (`self.GetActorBounds` (`|ConvertAsset` (`self.Floor`)) false))))
      (set `self.maxDistanceX` (.x (`.BoxExtent` (`self.GetActorBounds` (`|ConvertAsset` (`self.Floor`)) false)))))
    (:`then_1`
      ;;[1 1 1] Set and create HUD
      (bind _returnvalue (`|CreateWidget` "/Game/Blueprints/GUI/HUD.HUD_C"))
      (bind _output_get (set `self.HUD Reference` _returnvalue))
      (set `/Game/Blueprints/GUI/HUD.PlayerCameraPawn` self _output_get)
      (`UserWidget.AddToViewport` _output_get 0)
      (`Widget.SetVisibility` _output_get "Hidden"))
    (:`then_2`
      ;;[1 1 1] MiniMap actions
      (bind _outactors (`GameplayStatics.GetAllActorsOfClass` "/Game/PunkBoy/LP_miniMap_2_0.LP_miniMap_2_0_C" :!label _label))
      (`SceneComponent.K2_SetRelativeLocation` (`/Game/PunkBoy/LP_miniMap_2_0.MyCam` (`KismetArrayLibrary.Array_Get` _outactors)) (`KismetMathLibrary.MakeVector` _returnvalue_y _returnvalue_x 7000.0) false false))
    (:`then_3`
      ;;[1 1 1] Set and spawn ResourceManager
      (bind _returnvalue_2 (`|SpawnActorFromClass` "/Game/Blueprints/ResourceManagement/ResourceManager.ResourceManager_C" (`KismetMathLibrary.MakeTransform` (0.0 0.0 0.0)) "AlwaysSpawn" "OverrideRootScale"))
      (set `self.ResourceManagerRef` _returnvalue_2))))

(event `self.ReceiveTick`
  (params (DeltaSeconds :type "Float (single-precision)"))
  ;[1 1 1] BeginPlay operations
  ;;[1 1 1] MiniMap actions
  (goto _label))

(event `InputAxis|MoveForward`
  (params (AxisValue :type "Float (single-precision)"))
  ;[1 1 1] MOVE
  (if (`self.isMovingEnabled`) :!label _label_2
    (`self.CalculateAndSetActorTransform` (+ (`KismetMathLibrary.MakeVector` (* AxisValue (`self.MoveSpeed`))) (`KismetMathLibrary.MakeVector` 0.0 (* (stale `InputAxis|MoveRight` AxisValue) (`self.MoveSpeed`)))) self)))

(event `Key|MouseScrollUp`
  (params (Key :type "Key Structure" :default "AnyKey"))
  (bind _springarm (`self.SpringArm`))
  (bind _targetarmlength (`SpringArmComponent.TargetArmLength` _springarm))
  ;[1 1 1] ZOOM
  (:`Pressed`
    (if (> _targetarmlength (`self.minCameraHeight`))
      (set `SpringArmComponent.TargetArmLength` (- _targetarmlength (`self.ZoomSpeed`)) _springarm))))

(event `Key|LeftMouseButton`
  (params (Key :type "Key Structure" :default "AnyKey"))
  (bind _actorclass (`self.ActorClass`))
  (bind _spawnedactors (`self.SpawnedActors`))
  (bind (_worldlocation _worlddirection) (`PlayerController.DeprojectMousePositionToWorld` (`GameplayStatics.GetPlayerController` 0)))
  ;[1 1 1] SPAWNING ACTOR FROM CLASS
  (:`Pressed`
    (if (and (`self.isSpawningEnabled`) (!= _actorclass null))
      (set `self.isSpawningEnabled` false)
      (if (`/Game/Blueprints/ResourceManagement/ResourceManager.CanBuildActor` (`self.ResourceManagerRef`) _actorclass)
        (bind _asplayer_camera_pawn (cast `/Game/Blueprints/PlayerCameraPawn` (`GameplayStatics.GetPlayerPawn` 0)))
        (bind _outhit (`KismetSystemLibrary.LineTraceSingle` _worldlocation (+ _worldlocation (* _worlddirection (+ (`SpringArmComponent.TargetArmLength` (`/Game/Blueprints/PlayerCameraPawn.SpringArm` _asplayer_camera_pawn)) (`self.SightDistance`)))) "TraceTypeQuery3"))
        (bind (_bblockinghit _binitialoverlap _time _location _impactpoint _normal _impactnormal _physmat _hitactor) (`GameplayStatics.BreakHitResult` _outhit))
        (if (!= _hitactor null)
          (bind _returnvalue (`|SpawnActorFromClass` (`self.ActorClass`) (`KismetMathLibrary.Conv_VectorToTransform` (`KismetMathLibrary.MakeVector` (.x _location) (.y _location) 200.0)) "DontSpawnIfColliding" "OverrideRootScale"))
          (if (`KismetSystemLibrary.IsValid` _returnvalue)
            (`/Game/Blueprints/ResourceManagement/ResourceManager.UsingResourcesToBuildActor` (`self.ResourceManagerRef`) (`self.ActorClass`))
            (`KismetArrayLibrary.Array_Add` _spawnedactors _returnvalue)
            (`KismetSystemLibrary.PrintString` (`KismetStringLibrary.Concat_StrStr` "Spawned actors number: " (`KismetStringLibrary.Conv_IntToString` (`KismetArrayLibrary.Array_Length` _spawnedactors))) true true (struct :`R` 1.0 :`G` 0.153278 :`A` 1.0))
            (else
              (`KismetSystemLibrary.PrintString` "Collision detected, try another place!" true true (struct :`R` 1.0 :`A` 1.0))
              (set `self.ActorClass` null)
              (set `self.isSpawningEnabled` false))))
        (else
          (set `self.ActorClass` null)
          (set `self.isSpawningEnabled` false)))))
  (:`Released`
    (set `self.ActorClass` null)
    (set `self.isSpawningEnabled` false)))

(event `InputAxis|MoveRight`
  (params (AxisValue :type "Float (single-precision)"))
  ;[1 1 1] MOVE
  (goto _label_2))

(event `Key|MouseScrollDown`
  (params (Key :type "Key Structure" :default "AnyKey"))
  (bind _springarm (`self.SpringArm`))
  (bind _targetarmlength (`SpringArmComponent.TargetArmLength` _springarm))
  ;[1 1 1] ZOOM
  (:`Pressed`
    (if (< _targetarmlength (* (`self.zoom multiplyer`) (`self.minCameraHeight`)))
      (set `SpringArmComponent.TargetArmLength` (+ (`self.ZoomSpeed`) _targetarmlength) _springarm))))

(event `Key|One`
  (params (Key :type "Key Structure" :default "AnyKey"))
  ;[1 1 1] SPAWNING ACTOR FROM CLASS
)

(event `Key|Two`
  (params (Key :type "Key Structure" :default "AnyKey"))
  ;[1 1 1] SPAWNING ACTOR FROM CLASS
)

(event `InputAxisKey|MouseX`
  (params (AxisValue :type "Float (single-precision)"))
  ;[1 1 1] ROTATE
  (`/Engine/EditorBlueprintResources/StandardMacros.Gate` true :!label _label_3
    (:`Exit`
      (`self.K2_AddActorLocalRotation` (`KismetMathLibrary.MakeRotator` 0.0 0.0 (* (`self.RotateSpeed`) AxisValue))))))

(event `Key|RightMouseButton`
  (params (Key :type "Key Structure" :default "AnyKey"))
  (bind (_returnvalue_roll _returnvalue_pitch _returnvalue_yaw) (`KismetMathLibrary.BreakRotator` (`SceneComponent.K2_GetComponentRotation` (`self.Camera`))))
  ;[1 1 1] ROTATE
  (:`Pressed`
    (if (`self.isRotatingEnabled`)
      (set `self.isEdgeScrollingEnabled` false)
      (set `PlayerController.bShowMouseCursor` false (`GameplayStatics.GetPlayerController` 0))
      (`|ExecutionSequence`
        (:`then_0`
          (goto _label_3 :!via `Open`))
        (:`then_1`
          (goto _label_4 :!via `Open`)))))
  (:`Released`
    (set `self.isEdgeScrollingEnabled` true)
    (set `PlayerController.bShowMouseCursor` true (`GameplayStatics.GetPlayerController` 0))
    (`|ExecutionSequence`
      (:`then_0`
        (goto _label_3 :!via `Close`))
      (:`then_1`
        (goto _label_4 :!via `Close`)))))

(event `InputAxisKey|MouseY`
  (params (AxisValue :type "Float (single-precision)"))
  (bind (_returnvalue_roll _returnvalue_pitch _returnvalue_yaw) (`KismetMathLibrary.BreakRotator` (`SceneComponent.K2_GetComponentRotation` (`self.Camera`))))
  ;[1 1 1] ROTATE
  (`/Engine/EditorBlueprintResources/StandardMacros.Gate` true :!label _label_4
    (:`Exit`
      (`SceneComponent.K2_SetWorldRotation` (`self.Camera`) (`KismetMathLibrary.MakeRotator` _returnvalue_roll (`KismetMathLibrary.FClamp` (+ _returnvalue_pitch (* AxisValue (`self.RotateSpeed`))) -85.0 0.0) _returnvalue_yaw) false false))))

(event `InputAxisKey|MouseX`
  (params (AxisValue :type "Float (single-precision)"))
  (bind (_returnvalue_x _returnvalue_y) (`KismetMathLibrary.BreakVector2D` (`WidgetLayoutLibrary.GetViewportSize`)))
  (bind _movespeed (`self.MoveSpeed`))
  (bind _edgescrollarea (`self.EdgeScrollArea`))
  (bind _locationx (`PlayerController.GetMousePosition` (`GameplayStatics.GetPlayerController` 0)))
  ;[1 1 1] EDGE SCROLL
  (if (`self.isEdgeScrollingEnabled`)
    ;;[1 1 1] Scroll right
    (if (< (- _returnvalue_x _locationx) _edgescrollarea)
      (`self.CalculateAndSetActorTransform` (`KismetMathLibrary.MakeVector` 0.0 _movespeed) self)
      (else
        ;;[1 1 1] Scroll left
        (if (< _locationx _edgescrollarea)
          (`self.CalculateAndSetActorTransform` (`KismetMathLibrary.MakeVector` 0.0 (* _movespeed -1.0)) self))))))

(event `InputAxisKey|MouseY`
  (params (AxisValue :type "Float (single-precision)"))
  (bind (_returnvalue_x _returnvalue_y) (`KismetMathLibrary.BreakVector2D` (`WidgetLayoutLibrary.GetViewportSize`)))
  (bind _edgescrollarea (`self.EdgeScrollArea`))
  (bind _movespeed (`self.MoveSpeed`))
  (bind (_locationx _locationy) (`PlayerController.GetMousePosition` (`GameplayStatics.GetPlayerController` 0)))
  ;[1 1 1] EDGE SCROLL
  (if (`self.isEdgeScrollingEnabled`)
    ;;[1 1 1] Scroll down
    (if (< (- _returnvalue_y _locationy) _edgescrollarea)
      (`self.CalculateAndSetActorTransform` (`KismetMathLibrary.MakeVector` (* _movespeed -1.0)) self)
      (else
        ;;[1 1 1] Scroll up
        (if (< _locationy _edgescrollarea)
          (`self.CalculateAndSetActorTransform` (`KismetMathLibrary.MakeVector` _movespeed) self))))))

(fn `CalculateAndSetActorTransform`
  (params (MotionVector :type "Vector Structure") (Actor :type "Actor Object Reference"))
  (bind _returnvalue (`self.GetTransform` Actor))
  (bind _maxdistancex (`self.maxDistanceX`))
  (bind _maxdistancey (`self.maxDistanceY`))
  (`self.K2_SetActorTransform` Actor (`KismetMathLibrary.MakeTransform` (`KismetMathLibrary.MakeVector` (`KismetMathLibrary.FClamp` (.x (+ (`KismetMathLibrary.TransformDirection` _returnvalue MotionVector) (.location _returnvalue))) (* _maxdistancex -1.0) _maxdistancex) (`KismetMathLibrary.FClamp` (.y (+ (`KismetMathLibrary.TransformDirection` _returnvalue MotionVector) (.location _returnvalue))) (* _maxdistancey -1.0) _maxdistancey) (.z (+ (`KismetMathLibrary.TransformDirection` _returnvalue MotionVector) (.location _returnvalue)))) (.rotation _returnvalue) (.scale _returnvalue)) false false)
  (return))

(fn `UserConstructionScript`)