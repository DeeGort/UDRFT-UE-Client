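; ResourceAPI is a network Blueprint that reads the game's resources from a Firebase Realtime Database over its REST endpoints.
; Each resource type, such as Fruit, Iron or Wood, has its own getter with a hardcoded JSON URL on a test project.
; Every getter forwards its OnSuccess and OnFail callbacks to a shared GetResource call, whose body is not in this file.
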(fn `GetFruit`
  (params (`On Success` :type "Delegate (by ref)") (`On Fail` :type "Delegate (by ref)"))
  (`/Game/Blueprints/Network/NetworkAPI.GetResource` `On Success` `On Fail` "https://test-53f13.firebaseio.com/Fruit.json"))

(fn `GetIron`
  (params (`On Success` :type "Delegate (by ref)") (`On Fail` :type "Delegate (by ref)"))
  (`/Game/Blueprints/Network/NetworkAPI.GetResource` `On Success` `On Fail` "https://test-53f13.firebaseio.com/Iron.json"))

(fn `GetMeat`
  (params (`On Success` :type "Delegate (by ref)") (`On Fail` :type "Delegate (by ref)"))
  (`/Game/Blueprints/Network/NetworkAPI.GetResource` `On Success` `On Fail` "https://test-53f13.firebaseio.com/Meat.json"))

(fn `GetSand`
  (params (`On Success` :type "Delegate (by ref)") (`On Fail` :type "Delegate (by ref)"))
  (`/Game/Blueprints/Network/NetworkAPI.GetResource` `On Success` `On Fail` "https://test-53f13.firebaseio.com/Sand.json"))

(fn `GetStone`
  (params (`On Success` :type "Delegate (by ref)") (`On Fail` :type "Delegate (by ref)"))
  (`/Game/Blueprints/Network/NetworkAPI.GetResource` `On Success` `On Fail` "https://test-53f13.firebaseio.com/Stone.json"))

(fn `GetWater`
  (params (`On Success` :type "Delegate (by ref)") (`On Fail` :type "Delegate (by ref)"))
  (`/Game/Blueprints/Network/NetworkAPI.GetResource` `On Success` `On Fail` "https://test-53f13.firebaseio.com/Water.json"))

(fn `GetWheat`
  (params (`On Success` :type "Delegate (by ref)") (`On Fail` :type "Delegate (by ref)"))
  (`/Game/Blueprints/Network/NetworkAPI.GetResource` `On Success` `On Fail` "https://test-53f13.firebaseio.com/Wheat.json"))

(fn `GetWood`
  (params (`On Success` :type "Delegate (by ref)") (`On Fail` :type "Delegate (by ref)"))
  (`/Game/Blueprints/Network/NetworkAPI.GetResource` `On Success` `On Fail` "https://test-53f13.firebaseio.com/Wood.json"))