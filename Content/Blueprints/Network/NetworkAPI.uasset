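; NetworkAPI is a network helper that logs a user in by email and password through Google's Identity Toolkit verifyPassword REST endpoint.
; Login builds a JSON POST request, binds caller-supplied success and fail delegates, and fills the body with the credentials and a secure-token flag.
; It then sends the request to the endpoint URL, appended with a hardcoded API key.
; GetResource is an empty stub.
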(fn `GetResource`
  (params (URL :type String)))

(fn `Login`
  (params (`On Success` :type "Delegate (by ref)") (`On Fail` :type "Delegate (by ref)") (Username :type String) (Password :type String))
  (locals (Request :type "VaRestRequestJSON Object Reference") (`Parse Json Buffer` :type "VaRestJsonObject Object Reference") (`API key` :type String) (`Login URL` :type String))
  (bind _parse_json_buffer (`local.Parse Json Buffer`))
  (bind _output_get (set `local.Request` (`VaRestRequestJSON.ConstructRequestExt` "POST" "json")))
  (add `VaRestRequestJSON.OnRequestComplete` _output_get `On Success`)
  (add `VaRestRequestJSON.OnRequestFail` _output_get `On Fail`)
  (set `local.Parse Json Buffer` (`VaRestJsonObject.ConstructJsonObject`))
  (`VaRestJsonObject.SetStringField` _parse_json_buffer "email" Username)
  (`VaRestJsonObject.SetStringField` _parse_json_buffer "password" Password)
  (`VaRestJsonObject.SetStringField` _parse_json_buffer "returnSecureToken" "true")
  (`VaRestRequestJSON.SetRequestObject` (`local.Request`) _parse_json_buffer)
  (bind _output_get_2 (set `local.API key` "AIzaSyAaMOR2qRpNHPCkJ9r5mzkb5KSintfXd2c"))
  (bind _output_get_3 (set `local.Login URL` "https://www.googleapis.com/identitytoolkit/v3/relyingparty/verifyPassword"))
  (`VaRestRequestJSON.ProcessURL` (`local.Request`) (`KismetStringLibrary.Concat_StrStr` _output_get_3 "?key=" _output_get_2)))