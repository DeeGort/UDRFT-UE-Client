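; Resource manager that checks and deducts the costs of building test cottage and cube actors.
; The HUD, found through the player camera pawn, holds eight resource values that Tick copies into an index-based array.
; Cottage costs are compared and subtracted element-wise, with shortages printed in red, while cubes use only the HUD's stone value.
; After either deduction, the array is written back to the HUD.
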(event `self.ReceiveTick`
  (params (DeltaSeconds :type "Float (single-precision)"))
  (`self.GetHUDResources`))

(event `self.ReceiveBeginPlay`
  (`self.SetHUD_Ref`)
  (set `/Game/Blueprints/HUD.stoneValue` 50 (`self.Hud_Ref`)))

(fn `CanBuildActor`
  (params (ActorClass :type "Actor Class Reference"))
  (returns (HaveEnoughResources :type Boolean))
  (locals (Actor :type "Actor Class Reference") (isOK :type Boolean :default true))
  (set `local.Actor` ActorClass)
  ;[1 1 1] SwitchByActorClass
  (if (== (`local.Actor`) "/Game/Blueprints/BP_TestCottageActor.BP_TestCottageActor_C")
    ;[1 1 1] cottage
    (bind _isallgreaterorequal (`self.CompareArrays` (`self.Resources`) (`self.CottageResources`)))
    (if _isallgreaterorequal
      (set `self.isBuildingEnabled` true :!label _label)
      (else
        (`self.PrintResourceMessage` (`local.Actor`) (`self.CottageResources`) (`self.Resources`))
        (set `self.isBuildingEnabled` false :!label _label_2)))
    (elif (== (`local.Actor`) "/Game/Blueprints/BP_TestCubeActor.BP_TestCubeActor_C")
      ;[1 1 1] cube
      (if (>= (`/Game/Blueprints/HUD.stoneValue` (`self.HUD_Ref`)) (`self.CubeStoneResourceAmount`))
        (goto _label)
        (else
          (goto _label_2)))
      (elif (== (`local.Actor`) null)
        (goto _label_2)
        (else
          (`KismetSystemLibrary.PrintString` "IMPOSSIBLE ERROR" true true (struct :`R` 1.0 :`A` 1.0))
          (goto _label_2)))))
  (return (`self.isBuildingEnabled`)))

(fn `CompareArrays`
  (params (ResourceArray :type "Array of Integer") (BuildingResourceArray :type "Array of Integer"))
  (returns (isAllGreaterOrEqual :type Boolean))
  (locals (ok :type Boolean :default true))
  (for (_array_element _array_index) ResourceArray
    (set `local.ok` (and (>= _array_element (`KismetArrayLibrary.Array_Get` BuildingResourceArray _array_index)) (`local.ok`))))
  (return (`local.ok`)))

(fn `GetHUDResources`
  (bind _hud_ref (`self.Hud_Ref`))
  (`KismetArrayLibrary.Array_Set` (`self.Resources`) (`self.MeatIndex`) (`/Game/Blueprints/HUD.meatValue` _hud_ref))
  (`KismetArrayLibrary.Array_Set` (`self.Resources`) (`self.WaterIndex`) (`/Game/Blueprints/HUD.waterValue` _hud_ref))
  (`KismetArrayLibrary.Array_Set` (`self.Resources`) (`self.WheatIndex`) (`/Game/Blueprints/HUD.wheatValue` _hud_ref))
  (`KismetArrayLibrary.Array_Set` (`self.Resources`) (`self.FruitIndex`) (`/Game/Blueprints/HUD.fruitValue` _hud_ref))
  (`KismetArrayLibrary.Array_Set` (`self.Resources`) (`self.WoodIndex`) (`/Game/Blueprints/HUD.woodValue` _hud_ref))
  (`KismetArrayLibrary.Array_Set` (`self.Resources`) (`self.StoneIndex`) (`/Game/Blueprints/HUD.stoneValue` _hud_ref))
  (`KismetArrayLibrary.Array_Set` (`self.Resources`) (`self.IronIndex`) (`/Game/Blueprints/HUD.ironValue` _hud_ref))
  (`KismetArrayLibrary.Array_Set` (`self.Resources`) (`self.SandIndex`) (`/Game/Blueprints/HUD.sandValue` _hud_ref)))

(fn `PrintResourceMessage`
  (params (ActorClass :type "Actor Class Reference") (NeededResourcesArray :type "Array of Integer") (ResourcesArray :type "Array of Integer"))
  (locals (WoodString :type String) (StoneString :type String) (IronString :type String) (SandString :type String) (BuildingTypeString :type String) (DifferenceArray :type "Array of Integer") (ResStringArray :type "Array of String") (MeatString :type String) (WaterString :type String) (WheatString :type String) (FruitString :type String))
  (bind _resstringarray (`local.ResStringArray`))
  (bind _output_get (set `local.DifferenceArray` NeededResourcesArray))
  (`self.SubtractArrayElements` _output_get ResourcesArray
    (:`Completed`
      (for (_array_element _array_index) (`local.DifferenceArray`)
        (if (> _array_element 0)
          (`KismetArrayLibrary.Array_Set` _resstringarray _array_index (`KismetStringLibrary.Conv_IntToString` _array_element))))
      (for (_array_element_2 _array_index_2) _resstringarray
        (if (`KismetStringLibrary.NotEqual_StrStr` _array_element_2)
          (switch `int` _array_index_2
            (:`0`
              (set `local.MeatString` (`KismetStringLibrary.Concat_StrStr` _array_element_2 " more meat ")))
            (:`1`
              (set `local.WaterString` (`KismetStringLibrary.Concat_StrStr` _array_element_2 " more water ")))
            (:`2`
              (set `local.WheatString` (`KismetStringLibrary.Concat_StrStr` _array_element_2 " more wheat ")))
            (:`3`
              (set `local.FruitString` (`KismetStringLibrary.Concat_StrStr` _array_element_2 " more fruit ")))
            (:`4`
              (set `local.WoodString` (`KismetStringLibrary.Concat_StrStr` _array_element_2 " more wood ")))
            (:`5`
              (set `local.StoneString` (`KismetStringLibrary.Concat_StrStr` _array_element_2 " more stone ")))
            (:`6`
              (set `local.IronString` (`KismetStringLibrary.Concat_StrStr` _array_element_2 " more iron ")))
            (:`7`
              (set `local.SandString` (`KismetStringLibrary.Concat_StrStr` _array_element_2 " more sand "))))))
      (bind _buildingtype (`self.DefineBuildingType` ActorClass))
      (set `local.BuildingTypeString` _buildingtype)
      (`KismetSystemLibrary.PrintString` (`KismetStringLibrary.Concat_StrStr` "You need " (`local.MeatString`) (`local.WaterString`) (`local.WheatString`) (`local.FruitString`) (`local.WoodString`) (`local.StoneString`) (`local.IronString`) (`local.SandString`) " to make a " (`local.BuildingTypeString`) "!") true true (struct :`R` 1.0 :`A` 1.0) 10.0))))

(fn `UpdateHUDResources`
  (`self.SetHUD_Ref`)
  (`|ExecutionSequence`
    (:`then_0`
      (set `/Game/Blueprints/HUD.meatValue` (`KismetArrayLibrary.Array_Get` (`self.Resources`) (`self.MeatIndex`)) (`self.Hud_Ref`)))
    (:`then_1`
      (set `/Game/Blueprints/HUD.waterValue` (`KismetArrayLibrary.Array_Get` (`self.Resources`) (`self.WaterIndex`)) (`self.Hud_Ref`)))
    (:`then_2`
      (set `/Game/Blueprints/HUD.wheatValue` (`KismetArrayLibrary.Array_Get` (`self.Resources`) (`self.WheatIndex`)) (`self.Hud_Ref`)))
    (:`then_3`
      (set `/Game/Blueprints/HUD.fruitValue` (`KismetArrayLibrary.Array_Get` (`self.Resources`) (`self.FruitIndex`)) (`self.Hud_Ref`)))
    (:`then_4`
      (set `/Game/Blueprints/HUD.woodValue` (`KismetArrayLibrary.Array_Get` (`self.Resources`) (`self.WoodIndex`)) (`self.Hud_Ref`)))
    (:`then_5`
      (set `/Game/Blueprints/HUD.stoneValue` (`KismetArrayLibrary.Array_Get` (`self.Resources`) (`self.StoneIndex`)) (`self.Hud_Ref`)))
    (:`then_6`
      (set `/Game/Blueprints/HUD.ironValue` (`KismetArrayLibrary.Array_Get` (`self.Resources`) (`self.IronIndex`)) (`self.Hud_Ref`)))
    (:`then_7`
      (set `/Game/Blueprints/HUD.sandValue` (`KismetArrayLibrary.Array_Get` (`self.Resources`) (`self.SandIndex`)) (`self.Hud_Ref`)))))

(fn `UserConstructionScript`)

(fn `UsingResourcesToBuildActor`
  (params (ActorClass :type "Actor Class Reference"))
  (bind _hud_ref (`self.HUD_Ref`))
  ;[1 1 1] cottage resources
  (if (== ActorClass "/Game/Blueprints/BP_TestCottageActor.BP_TestCottageActor_C")
    (`self.SubtractArrayElements` (`self.Resources`) (`self.CottageResources`)
      (:`Completed`
        (`self.UpdateHUDResources` :!label _label)))
    (else
      ;[1 1 1] cube resources
      (if (== ActorClass "/Game/Blueprints/BP_TestCubeActor.BP_TestCubeActor_C")
        (set `/Game/Blueprints/HUD.stoneValue` (- (`/Game/Blueprints/HUD.stoneValue` _hud_ref) (`self.CubeStoneResourceAmount`)) _hud_ref)
        (goto _label)
        (elif (not (== ActorClass null))
          (`KismetSystemLibrary.PrintString` "IMPOSSIBLE ERROR" true true (struct :`R` 1.0 :`A` 1.0))))))
  (return))