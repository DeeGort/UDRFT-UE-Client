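; Placeable test cottage that follows the mouse as a preview plane until clicked, then becomes a cottage at that location.
; A Tick-fed gate, opened at BeginPlay, traces from the cursor and sweeps the actor to the clamped hit point at fixed height.
; Clicking closes the gate, logs the spawn once and clears the camera pawn's ActorClass.
; Hovering afterwards conditionally shows its selection marker, hiding those of other spawned cottages.
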(event `self.ReceiveBeginPlay`
  (bind (_worldlocation _worlddirection) (`PlayerController.DeprojectMousePositionToWorld` (`GameplayStatics.GetPlayerController` 0)))
  (`|ExecutionSequence`
    (:`then_0`
      (bind _asplayer_camera_pawn (cast `/Game/Blueprints/PlayerCameraPawn` (`GameplayStatics.GetPlayerPawn` 0)))
      (set `self.PlayerCameraPawnRef` _asplayer_camera_pawn))
    (:`then_1`
      (`SceneComponent.SetVisibility` (`self.Plane`) true false)
      (`SceneComponent.SetVisibility` (`self.Cottage`) false false)
      (goto _label :!via `Open`))))

(event `self.ReceiveActorOnReleased`
  (params (ButtonReleased :type "Key Structure" :default "AnyKey")))

(event `self.ReceiveTick`
  (params (DeltaSeconds :type "Float (single-precision)"))
  (bind (_worldlocation _worlddirection) (`PlayerController.DeprojectMousePositionToWorld` (`GameplayStatics.GetPlayerController` 0)))
  (`/Engine/EditorBlueprintResources/StandardMacros.Gate` true :!label _label
    (:`Exit`
      (bind _asplayer_camera_pawn (cast `/Game/Blueprints/PlayerCameraPawn` (`GameplayStatics.GetPlayerPawn` 0)))
      (bind (_outhit _returnvalue) (`KismetSystemLibrary.LineTraceSingle` _worldlocation (+ _worldlocation (* _worlddirection (+ (`SpringArmComponent.TargetArmLength` (`/Game/Blueprints/PlayerCameraPawn.SpringArm` _asplayer_camera_pawn)) (`/Game/Blueprints/PlayerCameraPawn.sightDistance` _asplayer_camera_pawn)))) "TraceTypeQuery3"))
      (if _returnvalue
        (`self.K2_SetActorLocation` (`KismetMathLibrary.MakeVector` (`KismetMathLibrary.FClamp` (.x (`.Location` (`GameplayStatics.BreakHitResult` _outhit))) -4000.0 4000.0) (`KismetMathLibrary.FClamp` (.y (`.Location` (`GameplayStatics.BreakHitResult` _outhit))) -4000.0 4000.0) 75.0) true)))))

(event `self.ReceiveActorOnClicked`
  (params (ButtonPressed :type "Key Structure" :default "AnyKey"))
  (`SceneComponent.SetVisibility` (`self.Plane`) false false)
  (`SceneComponent.SetVisibility` (`self.Cottage`) true false)
  (`|ExecutionSequence`
    (:`then_0`
      (goto _label :!via `Close`))
    (:`then_1`
      (if (not (`self.isPrintedSpawnInfo`))
        (`KismetSystemLibrary.PrintString` (`KismetStringLibrary.Concat_StrStr` "Spawned a Cottage at Location: " (`KismetStringLibrary.Conv_VectorToString` (`self.K2_GetActorLocation`))) true true (struct :`R` 0.87 :`G` 0.54681 :`A` 1.0) 10.0)
        (set `self.isPrintedSpawnInfo` true)
        (set `/Game/Blueprints/PlayerCameraPawn.ActorClass` null (`self.PlayerCameraPawnRef`))))))

(event `self.ReceiveActorBeginCursorOver`
  (bind _playercamerapawnref (`self.PlayerCameraPawnRef`))
  ;[1 1 1] selection
  (if (and (`self.isPrintedSpawnInfo`) (`/Game/Blueprints/PlayerCameraPawn.isEdgeScrollingEnabled` _playercamerapawnref) (== (`/Game/Blueprints/PlayerCameraPawn.ActorClass` _playercamerapawnref) null))
    (for _array_element (`/Game/Blueprints/PlayerCameraPawn.SpawnedActors` (`self.PlayerCameraPawnRef`))
      (if (== _array_element self)
        (bind _asbp_test_cottage_actor (cast `/Game/Blueprints/BP_TestCottageActor` _array_element))
        (`SceneComponent.SetVisibility` (`/Game/Blueprints/BP_TestCottageActor.Marker` _asbp_test_cottage_actor) true false)
        (`KismetSystemLibrary.PrintString` (`KismetStringLibrary.Concat_StrStr` (`KismetSystemLibrary.GetDisplayName` _asbp_test_cottage_actor) " is selected ") true true (struct :`G` 0.012906 :`B` 0.875 :`A` 1.0))
        (else
          (bind _asbp_test_cottage_actor_2 (cast `/Game/Blueprints/BP_TestCottageActor` _array_element))
          (`SceneComponent.SetVisibility` (`/Game/Blueprints/BP_TestCottageActor.Marker` _asbp_test_cottage_actor_2) false false))))))

(event `self.ReceiveActorEndCursorOver`
  ;[1 1 1] selection
  (`SceneComponent.SetVisibility` (`self.Marker`) false false))

(fn `UserConstructionScript`)